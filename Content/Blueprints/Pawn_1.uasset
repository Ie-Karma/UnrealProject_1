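; Pawn_1 is a basic player-controlled pawn that moves on the horizontal and vertical input axes, with a Left Shift sprint.
; Each Tick scales the actor's right and forward vectors by input, Speed and delta time, then applies a swept AddActorLocalOffset, feeding world-space vectors into a local-space move.
; Holding Left Shift doubles Speed until release.
; The AddMovementInput nodes are disconnected and never run.
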(event EventBeginPlay)

(event Collision|EventActorBeginOverlap
  (params (OtherActor :type Actor%20Object%20Reference)))

(event EventTick
  (params (DeltaSeconds :type Float%20%28single-precision%29))
  (bind _speed (Variables|Default|GetSpeed))
  ;[1 1 1] Movement
  (Transformation|AddActorLocalOffset (+ (* (Transformation|GetActorRightVector) (* (Input|AxisValues|GetHorizontal) DeltaSeconds _speed)) (* (* _speed DeltaSeconds (Input|AxisValues|GetVertical)) (Transformation|GetActorForwardVector))) true false))

(event Input|AxisEvents|InputAxisHorizontal
  (params (AxisValue :type Float%20%28single-precision%29))
  ;[1 1 1] Movement
)

(event Input|AxisEvents|InputAxisVertical
  (params (AxisValue :type Float%20%28single-precision%29))
  ;[1 1 1] Movement
)

(event Input|KeyboardEvents|LeftShift
  (params (Key :type Key%20Structure :default "None"))
  (:Pressed
    (Variables|Default|SetSpeed 1e+03))
  (:Released
    (Variables|Default|SetSpeed 5e+02)))

(event Input|KeyboardEvents|SpaceBar
  (params (Key :type Key%20Structure :default "None")))

(fn ConstructionScript)