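; Rotable is a component that continuously rotates its owning actor in timed steps.
; On BeginPlay it caches the owner's root component and world rotation, then starts a looping timer at a configurable interval.
; Each timer call adds the Incremento rotator to the stored rotation per axis, applies it in world space and saves the sum for the next step, leaving Tick unused.
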(event EventBeginPlay
  (Variables|Default|SetRootComponent (Variables|/Script/Engine.Actor|GetRootComponent (Components|GetOwner)))
  (Variables|Default|SetInitialRotation (Transformation|GetWorldRotation (Variables|/Script/Engine.Actor|GetRootComponent (Components|GetOwner))))
  (Utilities|Time|SetTimerbyFunctionName 0 "Rotate" (Variables|Default|GetTime) true))

(event EventTick
  (params (DeltaSeconds :type Float%20%28single-precision%29)))

(fn Rotate
  (bind _incremento (Variables|Default|GetIncremento))
  (Transformation|SetWorldRotation (Variables|Default|GetRootComponent) (Math|Rotator|MakeRotator (+ (.roll (Variables|Default|GetInitialRotation)) (.roll _incremento)) (+ (.pitch (Variables|Default|GetInitialRotation)) (.pitch _incremento)) (+ (.yaw (Variables|Default|GetInitialRotation)) (.yaw _incremento))) false false)
  (Variables|Default|SetInitialRotation (Math|Rotator|MakeRotator (+ (.roll (Variables|Default|GetInitialRotation)) (.roll _incremento)) (+ (.pitch (Variables|Default|GetInitialRotation)) (.pitch _incremento)) (+ (.yaw (Variables|Default|GetInitialRotation)) (.yaw _incremento)))))